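; Player character Blueprint, currently holding mostly test and debug scaffolding around inventory and interaction.
; BeginPlay adds a test reticle widget to the viewport, and a debug key drops global time dilation into slow motion.
; Tick prints the weapon inventory count from PlayerInventoryComponent.
; The interact input is empty, and prototype interaction checks (in-range actor listing, camera-angle look test, debug arrow) are left disconnected.
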(event Input|EnhancedActionEvents|EnhancedInputActionIA_PlayerInteract
  (params (ActionValue :type Boolean) (ElapsedSeconds :type Float%20%28double-precision%29) (TriggeredSeconds :type Float%20%28double-precision%29) (InputAction :type Input%20Action%20Object%20Reference :default "/Game/Core/Input/InputActions/IA_PlayerInteract.IA_PlayerInteract")))

(event EventTick
  (params (DeltaSeconds :type Float%20%28single-precision%29))
  ;[0.15 0.15 0.15 0.5] Testing logic used to determine if the player character is looking at an interactable object
  (Development|PrintString (Utilities|String|ToString(Integer) (Utilities|Array|Length (Variables|/Script/GPRProjectDelta.GPRInventoryComponentBase|GetWeaponInventoryArray (Variables|Default|GetPlayerInventoryComponent)))) true true "(R=0.000000,G=1.000000,B=0.016063,A=1.000000)" 0.0))

(event EventBeginPlay
  ;[0.15 0.15 0.15 0.5] Adds a reticle to the players screen for testing purposes
  (bind _returnvalue (UserInterface|CreateWidget "/Game/Blueprints/Widgets/WBP_TestReticle.WBP_TestReticle_C" (Game|GetPlayerController 0)))
  (UserInterface|Viewport|AddtoViewport _returnvalue 0))

(event Input|KeyboardEvents|DebugKeyT
  (params (Key :type Key%20Structure :default "None") (ActionValue :type Input%20Action%20Value%20Structure))
  (:Pressed
    (Utilities|Time|SetGlobalTimeDilation 0.1)))

(fn ConstructionScript)